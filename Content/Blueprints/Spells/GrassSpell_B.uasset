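; Grass spell actor built on a parent spell Blueprint, described as laying a circle of grass or foliage on the arena floor for combos with other spells.
; The construction script sets its stats, zero damage, description, and a type and name picked from inherited arrays.
; It passes speed and power to SetSpeed on the projectile movement, both there and again on BeginPlay.
; The file itself contains no foliage or combo logic.
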(event EventBeginPlay
  (|CallParentFunction)
  (CallFunction|SetSpeed (Variables|Default|GetSpeed) (Variables|Default|GetPower) (Variables|Default|GetProjectileMovement)))

(event Collision|EventActorBeginOverlap
  (params (OtherActor :type Actor%20Object%20Reference))
  (|CallParentFunction OtherActor) ; This node is disabled and will not be called.\nDrag off pins to build functionality.
)

(event EventTick
  (params (DeltaSeconds :type Float%20%28single-precision%29))
  (|CallParentFunction DeltaSeconds) ; This node is disabled and will not be called.\nDrag off pins to build functionality.
)

(fn ConstructionScript
  (|CallParentFunction)
  (Variables|Default|SetSpeed 100)
  (Variables|Default|SetPower 15)
  (Variables|Default|SetForce 5)
  (Variables|Default|SetDamage 0)
  (Variables|Default|SetDescription "A swarming mass of green, no bugs or ess. creates a circle of greass or foliage on the arena floor interacts with many of the spells but does not naturally generate flux initially but it can be comboed with other spells to have floor rated to reacting in order to unleash deadly combos.")
  (Variables|Default|SetType (Utilities|Array|Get(acopy) (Variables|Default|GetTypes) 3))
  (Variables|Default|SetName (Utilities|Array|Get(acopy) (Variables|Default|GetNames) 7))
  (CallFunction|SetSpeed (Variables|Default|GetSpeed) (Variables|Default|GetPower) (Variables|Default|GetProjectileMovement)))