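; Water spell projectile, a child spell Blueprint described in its text as an arcing ball of ocean that pushes back and soaks opponents.
; The construction script sets its stats, description, type and name, then passes speed and power to the inherited SetSpeed on ProjectileMovement.
; BeginPlay calls SetSpeed again after the parent logic.
; Overlap and Tick are disabled stubs, so no push or soak logic is implemented here.
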(event EventBeginPlay
  (|CallParentFunction)
  (CallFunction|SetSpeed (Variables|Default|GetSpeed) (Variables|Default|GetPower) (Variables|Default|GetProjectileMovement)))

(event Collision|EventActorBeginOverlap
  (params (OtherActor :type Actor%20Object%20Reference))
  (|CallParentFunction OtherActor) ; This node is disabled and will not be called.\nDrag off pins to build functionality.
)

(event EventTick
  (params (DeltaSeconds :type Float%20%28single-precision%29))
  (|CallParentFunction DeltaSeconds) ; This node is disabled and will not be called.\nDrag off pins to build functionality.
)

(fn ConstructionScript
  (|CallParentFunction)
  (Variables|Default|SetSpeed 50)
  (Variables|Default|SetPower 5)
  (Variables|Default|SetForce 200)
  (Variables|Default|SetDamage 10)
  (Variables|Default|SetDescription "A swirling ball of localised ocean. Thrown in an arc to push the opponent back and soak him in water. This can be utilized to push the opponent of the stage or possibly setup for electricity comebo as it would bounce off wet floors to create odd skill shots.")
  (Variables|Default|SetType (Utilities|Array|Get(acopy) (Variables|Default|GetTypes)))
  (Variables|Default|SetName (Utilities|Array|Get(acopy) (Variables|Default|GetNames) 6))
  (CallFunction|SetSpeed (Variables|Default|GetSpeed) (Variables|Default|GetPower) (Variables|Default|GetProjectileMovement)))