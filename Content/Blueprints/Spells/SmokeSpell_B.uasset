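; SmokeSpell_B is a spell projectile Blueprint, described as a held sphere of smoke that travels little and releases a large concealing cloud.
; Its construction script sets speed, power, force, zero damage, description, and a type and name picked from indexed arrays.
; Both construction and BeginPlay call SetSpeed to apply speed and power to the projectile movement component.
; The smoke, flux and fire behavior appears only in the description text, with no logic in these graphs.
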(event EventBeginPlay
  (|CallParentFunction)
  (CallFunction|SetSpeed (Variables|Default|GetSpeed) (Variables|Default|GetPower) (Variables|Default|GetProjectileMovement)))

(event Collision|EventActorBeginOverlap
  (params (OtherActor :type Actor%20Object%20Reference))
  (|CallParentFunction OtherActor) ; This node is disabled and will not be called.\nDrag off pins to build functionality.
)

(event EventTick
  (params (DeltaSeconds :type Float%20%28single-precision%29))
  (|CallParentFunction DeltaSeconds) ; This node is disabled and will not be called.\nDrag off pins to build functionality.
)

(fn ConstructionScript
  (|CallParentFunction)
  (Variables|Default|SetSpeed 1000)
  (Variables|Default|SetPower 150)
  (Variables|Default|SetForce 5)
  (Variables|Default|SetDamage 0)
  (Variables|Default|SetDescription "A barely contained sphere of smoke trapped in your hand. barely travels but hides you within a large body of smoke. Can be subterfuge and distracting purposes as flux can greatly expand. The area of smoke. Will also generate flux while the smoke is still fuming out but more sporadically than most so you need to get out of there before smoke leads to fire.")
  (Variables|Default|SetType (Utilities|Array|Get(acopy) (Variables|Default|GetTypes) 3))
  (Variables|Default|SetName (Utilities|Array|Get(acopy) (Variables|Default|GetNames) 4))
  (CallFunction|SetSpeed (Variables|Default|GetSpeed) (Variables|Default|GetPower) (Variables|Default|GetProjectileMovement)))