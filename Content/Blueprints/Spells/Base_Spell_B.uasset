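; Spell Blueprint Base_Spell_B, describing a faint, wobbling ball that flashes on contact, pushes opponents back and sheds flux as it travels.
; Its construction script runs the parent's, then sets name and type from indexed arrays, plus power, force, speed, damage, zero bounce and the description.
; The event graph holds only disabled stubs, so the behavior the description promises is not implemented in this Blueprint.
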(event EventBeginPlay
  (|CallParentFunction) ; This node is disabled and will not be called.\nDrag off pins to build functionality.
)

(event Collision|EventActorBeginOverlap
  (params (OtherActor :type Actor%20Object%20Reference))
  (|CallParentFunction OtherActor) ; This node is disabled and will not be called.\nDrag off pins to build functionality.
)

(event EventTick
  (params (DeltaSeconds :type Float%20%28single-precision%29))
  (|CallParentFunction DeltaSeconds) ; This node is disabled and will not be called.\nDrag off pins to build functionality.
)

(fn ConstructionScript
  (|CallParentFunction)
  (Variables|Default|SetName (Utilities|Array|Get(acopy) (Variables|Default|GetNames) 9))
  (Variables|Default|SetType (Utilities|Array|Get(acopy) (Variables|Default|GetTypes) 4))
  (Variables|Default|SetPower 10)
  (Variables|Default|SetForce 100)
  (Variables|Default|SetSpeed 150)
  (Variables|Default|SetDamage 25)
  (Variables|Default|SetBounce 0.0)
  (Variables|Default|SetDescription "A wobbling worryingly solid ball of almost nothing. Just the faintest hint at magic. Upon contact disperes in a flash of light and pushes opponent back. Drops a large amount of flux on travel making extremely useful for preping for more dangerous spells. Not suitable if it reached with anything but instead clears ground effects otherwise."))