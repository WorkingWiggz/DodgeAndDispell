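; EarthSpell is a projectile spell Blueprint that fills in spell stats and identity on top of inherited logic, though its description text describes a rolling ice ball.
; The construction script sets speed, power, force, damage and description, and picks its type and name from indexed arrays.
; SetSpeed applies speed and power to the ProjectileMovement component at construction and again on BeginPlay.
; It implements no overlap or tick logic of its own.
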(event EventBeginPlay
  (|CallParentFunction)
  (CallFunction|SetSpeed (Variables|Default|GetSpeed) (Variables|Default|GetPower) (Variables|Default|GetProjectileMovement)))

(event Collision|EventActorBeginOverlap
  (params (OtherActor :type Actor%20Object%20Reference))
  (|CallParentFunction OtherActor) ; This node is disabled and will not be called.\nDrag off pins to build functionality.
)

(event EventTick
  (params (DeltaSeconds :type Float%20%28single-precision%29))
  (|CallParentFunction DeltaSeconds) ; This node is disabled and will not be called.\nDrag off pins to build functionality.
)

(fn ConstructionScript
  (|CallParentFunction)
  (Variables|Default|SetSpeed 200)
  (Variables|Default|SetPower 50)
  (Variables|Default|SetForce 100)
  (Variables|Default|SetDamage 50)
  (Variables|Default|SetDescription "A thick frosted ball of ice, great for bowling penguins not so much people though, stopping or stunning opponents based on the closeness on impact but also give leeway in the form of a rolling moment to add for its lack of natural homing. not a huge amount of flux but can extend range and damage. ")
  (Variables|Default|SetType (Utilities|Array|Get(acopy) (Variables|Default|GetTypes) 1))
  (Variables|Default|SetName (Utilities|Array|Get(acopy) (Variables|Default|GetNames) 8))
  (CallFunction|SetSpeed (Variables|Default|GetSpeed) (Variables|Default|GetPower) (Variables|Default|GetProjectileMovement)))