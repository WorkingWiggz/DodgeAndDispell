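; Electric spell projectile, a child spell Blueprint described as a small, wildly arcing energy ball with low pushback.
; The construction script sets its speed, power, force, damage, description, and type and name from indexed arrays.
; SetSpeed applies speed and power to the ProjectileMovement component during construction and again on BeginPlay.
; The arcing, water bouncing and damage over time appear only in the description text, with no logic here.
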(event EventBeginPlay
  (|CallParentFunction)
  (CallFunction|SetSpeed (Variables|Default|GetSpeed) (Variables|Default|GetPower) (Variables|Default|GetProjectileMovement)))

(event Collision|EventActorBeginOverlap
  (params (OtherActor :type Actor%20Object%20Reference))
  (|CallParentFunction OtherActor) ; This node is disabled and will not be called.\nDrag off pins to build functionality.
)

(event EventTick
  (params (DeltaSeconds :type Float%20%28single-precision%29))
  (|CallParentFunction DeltaSeconds) ; This node is disabled and will not be called.\nDrag off pins to build functionality.
)

(fn ConstructionScript
  (|CallParentFunction)
  (Variables|Default|SetSpeed 100)
  (Variables|Default|SetPower 200)
  (Variables|Default|SetForce 100)
  (Variables|Default|SetDamage 10)
  (Variables|Default|SetDescription "A Small localized ball of energy. Arcs wildly towards target to an extent can bounce on water to extend range. on hit does damage initally and half of that on top across a few seconds not alot of push back however.")
  (Variables|Default|SetType (Utilities|Array|Get(acopy) (Variables|Default|GetTypes) 1))
  (Variables|Default|SetName (Utilities|Array|Get(acopy) (Variables|Default|GetNames) 1))
  (CallFunction|SetSpeed (Variables|Default|GetSpeed) (Variables|Default|GetPower) (Variables|Default|GetProjectileMovement)))