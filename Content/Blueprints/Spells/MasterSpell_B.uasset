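; MasterSpell_B is a spell actor that leaves element-specific Flux actors along its path and explodes on impact.
; Tick uses a Power-based Delay to throttle spawning, choosing the class by Name, though Electric spawns FireFlux_B.
; Hit scales Force and Damage spheres from their stats, then destroys the actor; sphere hits apply radial impulse and damage.
; FluxOverLap multiplies the selected Power, Force, Speed or Damage stat; its element switch is empty.
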(event OnComponentHit(ForceSphere)
  (params (HitComponent :type Primitive%20Component%20Object%20Reference) (OtherActor :type Actor%20Object%20Reference) (OtherComp :type Primitive%20Component%20Object%20Reference) (NormalImpulse :type Vector :default "0, 0, 0") (Hit :type Hit%20Result%20Structure%20%28by%20ref%29))
  (bind _forcesphere (Variables|Default|GetForceSphere))
  ;[1 1 1] Force impulse
  (Class|VisualLoggerKismetLibrary|LogText 0 "Force Hit" "VisLogBP")
  (Physics|AddRadialImpulse _forcesphere (Transformation|GetWorldLocation _forcesphere) (/ (.X (Math|Vector|BreakVector (Transformation|GetWorldScale _forcesphere))) 2.0) (+ (* (Variables|Default|GetForce) (Variables|Default|GetForceMulti)) (Math|Conversions|ToFloat(Integer) (Variables|Default|GetPower))) "RIF_Linear" false))

(event OnComponentHit(DamageSphere)
  (params (HitComponent :type Primitive%20Component%20Object%20Reference) (OtherActor :type Actor%20Object%20Reference) (OtherComp :type Primitive%20Component%20Object%20Reference) (NormalImpulse :type Vector :default "0, 0, 0") (Hit :type Hit%20Result%20Structure%20%28by%20ref%29))
  (bind _forcesphere (Variables|Default|GetForceSphere))
  ;[1 1 1] Damage Force
  (Class|VisualLoggerKismetLibrary|LogText 0 "DMG Hit" "VisLogBP")
  (Game|Damage|ApplyRadialDamage (Math|Conversions|ToFloat(Integer) (* (Variables|Default|GetPower) (Variables|Default|GetDamage))) (Transformation|GetWorldLocation _forcesphere) (.Y (Math|Vector|BreakVector (Transformation|GetWorldScale _forcesphere))) 0 0 (Components|GetOwner (Transformation|GetAttachParent (Variables|Default|GetDamageSphere))) 0 false "ECC_Visibility"))

(event Custom|ExplodeForce
  (bind _force (Variables|Default|GetForce))
  (bind _forcemulti (Variables|Default|GetForceMulti))
  (bind _returnvalue (* _force _forcemulti))
  ;[1 1 1] Explode Force Sphere
  (Transformation|SetWorldScale3D (Variables|Default|GetForceSphere) (Math|Interpolation|Ease :Function "Linear" :Alpha 0.5 :B (Math|Vector|MakeVector _returnvalue _returnvalue _returnvalue))))

(event Custom|ExplodeDamage
  (bind _damage (Variables|Default|GetDamage))
  (bind _damagemulti (Variables|Default|GetDamageMulti))
  (bind _returnvalue (* _damage _damagemulti))
  ;[1 1 1] Expand Damage Sphere
  (Transformation|SetWorldScale3D (Variables|Default|GetDamageSphere) (Math|Interpolation|Ease :Function "Linear" :Alpha 0.5 :B (Math|Vector|MakeVector _returnvalue _returnvalue _returnvalue))))

(event EventBeginPlay)

(event EventTick
  (params (DeltaSeconds :type Float%20%28single-precision%29))
  ;[1 1 1] Spawn Flux Actors depending on name each tick
  (Utilities|FlowControl|Delay (Math|Conversions|ToFloat(Integer) (/ (Variables|Default|GetPower) 100)))
  (switch string (Variables|Default|GetName)
    (:Fire
      (Game|SpawnActorfromClass "/Game/Blueprints/Flux/FireFlux_B.FireFlux_B_C" (Transformation|GetActorTransform self) "AdjustIfPossibleButAlwaysSpawn" 0 0))
    (:Ice
      (Game|SpawnActorfromClass "/Game/Blueprints/Flux/IceFlux_B.IceFlux_B_C" (Transformation|GetActorTransform self) "AdjustIfPossibleButAlwaysSpawn" 0 0))
    (:Electric
      (Game|SpawnActorfromClass "/Game/Blueprints/Flux/FireFlux_B.FireFlux_B_C" (Transformation|GetActorTransform self) "AdjustIfPossibleButAlwaysSpawn" 0 0))
    (:Slime
      (Game|SpawnActorfromClass "/Game/Blueprints/Flux/SlimeFlux_B.SlimeFlux_B_C" (Transformation|GetActorTransform self) "AdjustIfPossibleButAlwaysSpawn" 0 0))
    (:Smoke
      (Game|SpawnActorfromClass "/Game/Blueprints/Flux/SmokeFlux_B.SmokeFlux_B_C" (Transformation|GetActorTransform self) "AdjustIfPossibleButAlwaysSpawn" 0 0))
    (:Water
      (Game|SpawnActorfromClass "/Game/Blueprints/Flux/WaterFlux_B.WaterFlux_B_C" (Transformation|GetActorTransform self) "AdjustIfPossibleButAlwaysSpawn" 0 0))
    (:Base
      (Game|SpawnActorfromClass "/Game/Blueprints/Flux/BaseFlux_B.BaseFlux_B_C" (Transformation|GetActorTransform self) "AdjustIfPossibleButAlwaysSpawn" 0 0))
    (:Earth
      (Game|SpawnActorfromClass "/Game/Blueprints/Flux/EarthFlux_B.EarthFlux_B_C" (Transformation|GetActorTransform self) "AdjustIfPossibleButAlwaysSpawn" 0 0))
    (:Grass
      (Game|SpawnActorfromClass "/Game/Blueprints/Flux/GrassFlux_B.GrassFlux_B_C" (Transformation|GetActorTransform self) "AdjustIfPossibleButAlwaysSpawn" 0 0))
    (:Poison
      (Game|SpawnActorfromClass "/Game/Blueprints/Flux/PoisonFlux_B.PoisonFlux_B_C" (Transformation|GetActorTransform self) "AdjustIfPossibleButAlwaysSpawn" 0 0))))

(event Collision|EventHit
  (params (MyComp :type Primitive%20Component%20Object%20Reference) (Other :type Actor%20Object%20Reference) (OtherComp :type Primitive%20Component%20Object%20Reference) (bSelfMoved :type Boolean) (HitLocation :type Vector :default "0, 0, 0") (HitNormal :type Vector :default "0, 0, 0") (NormalImpulse :type Vector :default "0, 0, 0") (Hit :type Hit%20Result%20Structure%20%28by%20ref%29))
  ;[1 1 1] On Collision with solid object, destroy object after creating explosion
  (CallFunction|ExplodeForce)
  (CallFunction|ExplodeDamage)
  (Actor|DestroyActor))

(fn ConstructionScript)

(fn FluxOverLap
  (params (FluxN :type Name) (FluxE :type Name) (Multi :type Float%20%28single-precision%29))
  (switch name FluxE
    (:Power
      (Variables|Default|SetPower (Math|Float|Round (* (Variables|Default|GetPower) Multi))))
    (:Force
      (Variables|Default|SetForce (Math|Float|Round (* (Variables|Default|GetForce) Multi))))
    (:Speed
      (Variables|Default|SetSpeed (Math|Float|Round (* (Variables|Default|GetSpeed) Multi))))
    (:Damage
      (Variables|Default|SetDamage (Math|Float|Round (* (Variables|Default|GetDamage) Multi)))))
  (switch name FluxN))